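; Puzzle game mode that tracks pickup totals, score and combo state.
; Addscore awards points for the first three pickups in a sequence and pulses timed combo flags; ResetScore restarts the sequence.
; SetComboOn opens a two-second combo window, and turn4xCombo triggers the x4 flag without scoring.
; The input-sequence combo check is disconnected, and the per-tick Test on the cached player does nothing.
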(event Custom|Test
  (if (Variables|/Game/PuzzleGame/Blueprints/PuzzlePlayer.PuzzlePlayer_C|GetLmbDown (Variables|Default|GetPlayer))
    _))

(event Custom|turn4xCombo
  (Variables|Default|SetisX2Combo false)
  (Variables|Default|SetisX4Combo true)
  (Utilities|FlowControl|Delay 2.0)
  (Variables|Default|SetisX4Combo false))

(event Custom|Add%20score
  (Variables|Default|SetPickUpsTotal (+ (Variables|Default|GetPickUpsTotal) 1.0))
  (Variables|Default|SetScorePickUpSequence (+ (Variables|Default|GetScorePickUpSequence) 1.0))
  (if (== (Variables|Default|GetScorePickUpSequence) 1.0)
    (Variables|Default|SetScore (+ (Variables|Default|GetScore) (Variables|Default|GetScorePickUp_Normal)))
    (Variables|Default|SetisX1Combo true)
    (Utilities|FlowControl|Delay 2.0)
    (Variables|Default|SetisX1Combo false)
    (elif (== (Variables|Default|GetScorePickUpSequence) 2.0)
      (Variables|Default|SetScore (+ (Variables|Default|GetScore) (Variables|Default|GetScorePickUp_Combox1)))
      (Variables|Default|SetisX2Combo true)
      (Utilities|FlowControl|Delay 2.0)
      (Variables|Default|SetisX2Combo false)
      (elif (== (Variables|Default|GetScorePickUpSequence) 3.0)
        (Variables|Default|SetScore (+ (Variables|Default|GetScore) (Variables|Default|GetScorePickUp_Combox2)))
        (Variables|Default|SetisX2Combo false)
        (Variables|Default|SetisX4Combo true)
        (Utilities|FlowControl|Delay 2.0)
        (Variables|Default|SetisX4Combo false)))))

(event Custom|SetComboOn
  (Variables|Default|SetComboOn true)
  (Utilities|FlowControl|Delay 2.0)
  (Variables|Default|SetComboOn false)
  (Variables|Default|SetHasBeenPickedOneTime false))

(event Custom|Reset%20Score
  (Variables|Default|SetScorePickUpSequence 0.0))

(event EventTick
  (params (DeltaSeconds :type Float%20%28single-precision%29))
  (CallFunction|Test))

(event EventBeginPlay
  ;[1 1 1] Get Player Reference
  (bind _aspuzzle_player (Utilities|Casting|CastToPuzzlePlayer (Pawn|GetControlledPawn (Game|GetPlayerController 0))))
  (Variables|Default|SetPlayer _aspuzzle_player))

(fn ConstructionScript)

(fn CheckCombo)

(fn CheckComboSimple)