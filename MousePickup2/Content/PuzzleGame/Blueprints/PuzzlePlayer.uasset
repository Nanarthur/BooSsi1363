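; PuzzlePlayer is the player camera for the puzzle game, with mouse-driven zoom and panning inside set bounds.
; The wheel moves it along the camera's forward vector, and right-button drag pans it in world X and Y, both feeding a shared location clamp.
; Paired DoOnce nodes track left and right button state, though the left state is not read here.
; The construction script centers it within the bounds.
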(event Input|MouseEvents|MouseX
  (params (AxisValue :type Float%20%28single-precision%29))
  (bind _returnvalue (Transformation|GetActorLocation))
  (bind _cameraboundsx (Variables|Default|GetCameraBoundsX))
  (bind _cameraboundsy (Variables|Default|GetCameraBoundsY))
  (bind _cameraboundsz (Variables|Default|GetCameraBoundsZ))
  ;[1 1 1] Camera Panning
  (if (Variables|Default|GetRmbDown)
    (Transformation|AddActorWorldOffset (Math|Vector|MakeVector (* (* AxisValue (Variables|Default|GetCameraPanSpeed)) -1.0) 0.0 0.0))
    ;[1 1 1] Clamp Camera Location
    (Transformation|SetActorLocation (Math|Vector|MakeVector (Math|Float|Clamp(Float) (.x _returnvalue) (.x _cameraboundsx) (.y _cameraboundsx)) (Math|Float|Clamp(Float) (.y _returnvalue) (.x _cameraboundsy) (.y _cameraboundsy)) (Math|Float|Clamp(Float) (.z _returnvalue) (.x _cameraboundsz) (.y _cameraboundsz))) false false)))

(event Input|MouseEvents|MouseY
  (params (AxisValue :type Float%20%28single-precision%29))
  (bind _returnvalue (Transformation|GetActorLocation))
  (bind _cameraboundsx (Variables|Default|GetCameraBoundsX))
  (bind _cameraboundsy (Variables|Default|GetCameraBoundsY))
  (bind _cameraboundsz (Variables|Default|GetCameraBoundsZ))
  ;[1 1 1] Camera Panning
  (if (Variables|Default|GetRmbDown)
    (Transformation|AddActorWorldOffset (Math|Vector|MakeVector 0.0 (* (Variables|Default|GetCameraPanSpeed) AxisValue) 0.0))
    ;[1 1 1] Clamp Camera Location
    (Transformation|SetActorLocation (Math|Vector|MakeVector (Math|Float|Clamp(Float) (.x _returnvalue) (.x _cameraboundsx) (.y _cameraboundsx)) (Math|Float|Clamp(Float) (.y _returnvalue) (.x _cameraboundsy) (.y _cameraboundsy)) (Math|Float|Clamp(Float) (.z _returnvalue) (.x _cameraboundsz) (.y _cameraboundsz))) false false)))

(event Input|MouseEvents|MouseWheelAxis
  (params (AxisValue :type Float%20%28single-precision%29))
  (bind _returnvalue (Transformation|GetActorLocation))
  (bind _cameraboundsx (Variables|Default|GetCameraBoundsX))
  (bind _cameraboundsy (Variables|Default|GetCameraBoundsY))
  (bind _cameraboundsz (Variables|Default|GetCameraBoundsZ))
  ;[1 1 1] Camera Zoom
  (Transformation|AddActorWorldOffset (* (Math|Vector|GetForwardVector (Variables|Default|GetCamera)) (* AxisValue (Variables|Default|GetCameraZoomSpeed))))
  ;[1 1 1] Clamp Camera Location
  (Transformation|SetActorLocation (Math|Vector|MakeVector (Math|Float|Clamp(Float) (.x _returnvalue) (.x _cameraboundsx) (.y _cameraboundsx)) (Math|Float|Clamp(Float) (.y _returnvalue) (.x _cameraboundsy) (.y _cameraboundsy)) (Math|Float|Clamp(Float) (.z _returnvalue) (.x _cameraboundsz) (.y _cameraboundsz))) false false))

(event Input|MouseEvents|RightMouseButton
  (params (Key :type Key%20Structure :default "AnyKey"))
  ;[1 1 1] Mouse Buttons
  (:Pressed
    (Utilities|FlowControl|DoOnce false :!label _label
      (:Completed
        (Variables|Default|SetRmbDown true)
        (goto _label_2 Reset))))
  (:Released
    (Utilities|FlowControl|DoOnce true :!label _label_2
      (:Completed
        (Variables|Default|SetRmbDown false)
        (goto _label Reset)))))

(event Input|MouseEvents|LeftMouseButton
  (params (Key :type Key%20Structure :default "AnyKey"))
  ;[1 1 1] Mouse Buttons
  (:Pressed
    (Utilities|FlowControl|DoOnce false :!label _label
      (:Completed
        (Variables|Default|SetLmbDown true)
        (goto _label_2 Reset))))
  (:Released
    (Utilities|FlowControl|DoOnce true :!label _label_2
      (:Completed
        (Variables|Default|SetLmbDown false)
        (goto _label Reset)))))

(fn ConstructionScript
  (bind _cameraboundsx (Variables|Default|GetCameraBoundsX))
  (bind _cameraboundsz (Variables|Default|GetCameraBoundsZ))
  (bind _cameraboundsy (Variables|Default|GetCameraBoundsY))
  (Transformation|SetActorLocation (Math|Vector|MakeVector (Math|Float|Lerp (.x _cameraboundsx) (.y _cameraboundsx) 0.5) (Math|Float|Lerp (.x _cameraboundsy) (.y _cameraboundsy) 0.5) (Math|Float|Lerp (.x _cameraboundsz) (.y _cameraboundsz) 0.5)) false false))