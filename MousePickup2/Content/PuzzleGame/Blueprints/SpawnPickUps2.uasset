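; SpawnPickUps2 is a puzzle pickup that feeds the digit "2" into the game mode's combo input.
; When a PuzzlePiece overlaps its Box, it appends the digit to PuzzleGameMode's ComboInput, adds score and destroys its Cube, Box and Number components.
; The index returned by the append triggers CheckCombo when it equals 2, meaning this pickup supplied the third entry.
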(event OnComponentBeginOverlap(Box)
  (params (OverlappedComponent :type Primitive%20Component%20Object%20Reference) (OtherActor :type Actor%20Object%20Reference) (OtherComp :type Primitive%20Component%20Object%20Reference) (OtherBodyIndex :type Integer) (bFromSweep :type Boolean) (SweepResult :type Hit%20Result%20Structure%20%28by%20ref%29))
  (Utilities|Casting|CastToPuzzlePiece OtherActor)
  (bind _aspuzzle_game_mode (Utilities|Casting|CastToPuzzleGameMode (Game|GetGameMode)))
  (bind _returnvalue (Utilities|Array|Add (Variables|/Game/PuzzleGame/Blueprints/PuzzleGameMode.PuzzleGameMode_C|GetComboInput _aspuzzle_game_mode) (Utilities|Text|MakeLiteralText "2")))
  (Default|AddScore _aspuzzle_game_mode)
  (Components|DestroyComponent (Variables|Default|GetCube))
  (if (== _returnvalue 2)
    (Default|CheckCombo _aspuzzle_game_mode)))

(event EventBeginPlay)

(fn ConstructionScript)