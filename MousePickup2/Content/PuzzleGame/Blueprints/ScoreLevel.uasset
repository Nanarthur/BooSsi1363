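; ScoreLevel is the puzzle game's in-world score display, with text pop-ups for combo bonuses.
; BeginPlay seeds the PuzzleGameMode score from its ScoreLevel value.
; Tick polls the game mode, refreshing the score text and checking the X4, X2 and X1 combo flags to fire +200, +100 and +50 events.
; Each event reveals its TextRender for two seconds; the two larger bonuses also hide the other pop-ups.
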(event Custom|show+50
  (bind _textrender3 (Variables|Default|GetTextRender3))
  (Rendering|SetVisibility _textrender3 true false)
  (Utilities|FlowControl|Delay 2.0)
  (Rendering|SetVisibility _textrender3 false false))

(event Custom|show+200
  (bind _textrender2 (Variables|Default|GetTextRender2))
  (Rendering|SetVisibility (Variables|Default|GetTextRender3) false false)
  (Rendering|SetVisibility _textrender2 true false)
  (Utilities|FlowControl|Delay 2.0)
  (Rendering|SetVisibility _textrender2 false false))

(event Custom|show+100
  (bind _textrender1 (Variables|Default|GetTextRender1))
  (Rendering|SetVisibility (Variables|Default|GetTextRender3) false false)
  (Rendering|SetVisibility _textrender1 true false)
  (Utilities|FlowControl|Delay 2.0)
  (Rendering|SetVisibility _textrender1 false false))

(event EventBeginPlay
  (bind _aspuzzle_game_mode (Utilities|Casting|CastToPuzzleGameMode (Game|GetGameMode)))
  (Variables|/Game/PuzzleGame/Blueprints/PuzzleGameMode.PuzzleGameMode_C|SetScore _aspuzzle_game_mode (Variables|Default|GetScoreLevel)))

(event EventTick
  (params (DeltaSeconds :type Float%20%28single-precision%29))
  (bind _aspuzzle_game_mode (Utilities|Casting|CastToPuzzleGameMode (Game|GetGameMode)))
  (Rendering|Components|TextRender|SetText (Variables|Default|GetTextRender) (Utilities|Text|ToText(Float) (Variables|/Game/PuzzleGame/Blueprints/PuzzleGameMode.PuzzleGameMode_C|GetScore _aspuzzle_game_mode) "HalfToEven"))
  (Utilities|FlowControl|Sequence
    (:then_0
      (if (Variables|/Game/PuzzleGame/Blueprints/PuzzleGameMode.PuzzleGameMode_C|GetisX4Combo _aspuzzle_game_mode)
        (CallFunction|Show+200)
        (else
          (if (Variables|/Game/PuzzleGame/Blueprints/PuzzleGameMode.PuzzleGameMode_C|GetisX1Combo _aspuzzle_game_mode) :!label _label
            (CallFunction|Show+50)))))
    (:then_1
      (if (Variables|/Game/PuzzleGame/Blueprints/PuzzleGameMode.PuzzleGameMode_C|GetisX2Combo _aspuzzle_game_mode)
        (CallFunction|Show+100)
        (else
          (goto _label))))))

(fn ConstructionScript)