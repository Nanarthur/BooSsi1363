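; Puzzle piece actor that the player drags with the mouse, tinted per instance through a dynamic material.
; Holding LMB over it disables physics, resets the game mode score and sweeps the piece to the cursor trace hit each Tick.
; When not held it simulates physics and flags sliding from its speed, but the sliding score events are empty.
; Death disables input, hides the mesh and spawns an explosion effect with sound.
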(event Custom|Pick%20Up%20Mesh
  (bind _returnvalue (Game|GetPlayerController 0))
  (bind (_worldlocation _worlddirection) (Game|Player|ConvertMouseLocationToWorldSpace _returnvalue))
  ;[1 1 1] Attach to cursor
  (if (Variables|Default|GetAttached%20To%20Cursor)
    (bind (_outhit _returnvalue_2) (Collision|LineTraceByChannel _worldlocation (+ _worldlocation (* _worlddirection (Variables|Default|GetCursor%20Trace%20Distance))) "TraceTypeQuery3" false 0 "None"))
    (if _returnvalue_2
      (Transformation|SetActorLocation (+ (.Location (Collision|BreakHitResult _outhit)) "0, 0,5.000000") true false))))

(event Custom|AddScoreIfSliding)

(event Custom|IsMoving
  (if (not (and (Variables|Default|GetCursor%20Hover) (Variables|/Game/PuzzleGame/Blueprints/PuzzlePlayer.PuzzlePlayer_C|GetLmbDown (Variables|Default|GetPlayer))))
    (if (> (Math|Vector|VectorLength (Transformation|GetVelocity)) 5e+01)
      (Variables|Default|SetIsSliding true)
      (else
        (Variables|Default|SetIsSliding false)))))

(event Custom|Add%20Score)

(event Custom|Check%20Attach
  ;[1 1 1] Check if should attach to cursor
  (if (and (Variables|Default|GetCursor%20Hover) (Variables|/Game/PuzzleGame/Blueprints/PuzzlePlayer.PuzzlePlayer_C|GetLmbDown (Variables|Default|GetPlayer)))
    (CallFunction|SetAttached true)
    (bind _aspuzzle_game_mode (Utilities|Casting|CastToPuzzleGameMode (Game|GetGameMode)))
    (Default|ResetScore _aspuzzle_game_mode)
    (else
      (CallFunction|SetAttached false))))

(event Custom|Death
  (bind _returnvalue (Transformation|GetActorLocation))
  (Variables|Default|SetIsDead true)
  (Input|DisableInput 0)
  (Effects|SpawnEmitteratLocation "/Game/MobileStarterContent/Particles/P_Explosion.P_Explosion" _returnvalue)
  (Audio|SpawnSoundatLocation "/Game/MobileStarterContent/Audio/Explosion01.Explosion01" _returnvalue)
  (Rendering|SetVisibility (Variables|Default|GetPiece) false false))

(event EventBeginPlay
  ;[1 1 1] Get Player Reference
  (bind _aspuzzle_player (Utilities|Casting|CastToPuzzlePlayer (Pawn|GetControlledPawn (Game|GetPlayerController 0))))
  (Variables|Default|SetPlayer _aspuzzle_player))

(event MouseInput|EventActorBeginCursorOver
  ;[1 1 1] Cursor Hover State
  (Variables|Default|SetCursor%20Hover true))

(event MouseInput|EventActorEndCursorOver
  ;[1 1 1] Cursor Hover State
  (Variables|Default|SetCursor%20Hover false))

(event EventTick
  (params (DeltaSeconds :type Float%20%28single-precision%29))
  ;[1 1 1] Tick
  (CallFunction|CheckAttach)
  (CallFunction|PickUpMesh)
  (CallFunction|IsMoving)
  (CallFunction|AddScoreifSliding))

(fn ConstructionScript
  (bind _piece (Variables|Default|GetPiece))
  (bind _returnvalue (Rendering|Material|CreateDynamicMaterialInstance _piece 0 "/Game/PuzzleGame/Materials/M_PuzzlePiece.M_PuzzlePiece" :!class /Script/Engine.PrimitiveComponent))
  (Rendering|Material|SetVectorParameterValue _returnvalue "Color" (Variables|Default|GetColor) :!class /Script/Engine.MaterialInstanceDynamic)
  (Rendering|Material|SetMaterial _piece 0 _returnvalue))

(fn SetAttached
  (params (Attached :type Boolean))
  (Physics|SetSimulatePhysics (Variables|Default|GetPiece) (not Attached))
  (Variables|Default|SetAttached%20To%20Cursor Attached))